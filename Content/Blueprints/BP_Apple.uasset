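; BP_Apple is a falling apple pickup for an apple-picker game.
; Any actor overlap destroys it.
; On Tick, once its sphere collider drops below MaximumFallDistance, it tells the ApplePickerGameState to fire the basket damage dispatcher, then destroys itself.
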(event EventBeginPlay)

(event Collision|EventActorBeginOverlap
  (params (OtherActor :type Actor%20Object%20Reference))
  (Actor|DestroyActor))

(event EventTick
  (params (DeltaSeconds :type Float%20%28single-precision%29))
  (if (< (.z (Transformation|GetWorldLocation (Variables|Default|GetSphere%20Collider))) (Variables|Default|GetMaximumFallDistance))
    (bind _asapple_picker_game_state (Utilities|Casting|CastToApplePickerGameState (Game|GetGameState)))
    (Default|CallBasketDamageDispatcher _asapple_picker_game_state)
    (Actor|DestroyActor)))

(fn ConstructionScript)