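; Player-controlled basket for an apple picker game that slides horizontally to score on overlaps and loses stacked basket components when damaged.
; Enhanced Input drives Move, which scales input by speed and stored Tick delta time, then sweeps along X only within Bounds.
; Overlaps fire the game state's score dispatcher.
; Its damage dispatcher destroys one basket component per hit, or reloads the Picker level when health is depleted.
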(event Custom|Event%20OnDamage
  (if (> (Variables|Default|GetHealth) 0)
    (bind _result (Math|Integer|DecrementInt (Variables|Default|GetHealth))
      (:%20%20
        (Components|DestroyComponent (Utilities|Array|Get(acopy) (Variables|Default|GetBaskets) _result))
        (Variables|Default|SetHealth (- (Variables|Default|GetHealth) 1))))
    (else
      (Game|OpenLevel(byObjectReference) "/Game/Levels/Picker.Picker"))))

(event Input|EnhancedActionEvents|EnhancedInputActionIA_Move
  (params (ActionValue :type Float%20%28double-precision%29) (ElapsedSeconds :type Float%20%28double-precision%29) (TriggeredSeconds :type Float%20%28double-precision%29) (InputAction :type Input%20Action%20Object%20Reference :default "/Game/Input/IA_Move.IA_Move"))
  (CallFunction|Move ActionValue))

(event EventBeginPlay
  (CallFunction|SetupInput)
  (CallFunction|SetupBaskets)
  (bind _asapple_picker_game_state (Utilities|Casting|CastToApplePickerGameState (Game|GetGameState)))
  (EventDispatchers|BindEventtoBasketDamageDispatcher _asapple_picker_game_state (delegate Custom|Event%20OnDamage)))

(event Collision|EventActorBeginOverlap
  (params (OtherActor :type Actor%20Object%20Reference))
  (bind _asapple_picker_game_state (Utilities|Casting|CastToApplePickerGameState (Game|GetGameState)))
  (Default|CallAddScoreDispatcher _asapple_picker_game_state))

(event EventTick
  (params (DeltaSeconds :type Float%20%28single-precision%29))
  (Variables|Default|SetDeltaTime DeltaSeconds))

(fn ConstructionScript)

(fn Move
  (params (Input :type Float%20%28double-precision%29))
  (bind _returnvalue (Transformation|GetActorLocation))
  (bind _deltatime (Variables|Default|GetDeltaTime))
  (bind _speed (Variables|Default|GetSpeed))
  (bind _returnvalue_2 (* Input _speed))
  (bind _returnvalue_3 (* _returnvalue_2 _deltatime))
  (bind _returnvalue_4 (Math|Vector|MakeVector _returnvalue_3 0.0 0.0))
  (bind _returnvalue_5 (+ _returnvalue_4 _returnvalue))
  (bind _canmove (CallFunction|CanMove (.x _returnvalue_5)))
  (if _canmove
    (Transformation|SetActorLocation (Math|Vector|MakeVector (.x _returnvalue_5) (.y _returnvalue_5) (.z _returnvalue_5)) true false)))

(fn CanMove
  (params (Position :type Float%20%28double-precision%29))
  (return (not (or (> Position (.y (Variables|Default|GetBounds))) (< Position (.x (Variables|Default|GetBounds)))))))

(fn SetupInput
  (bind _asplayer_controller (Utilities|Casting|CastToPlayerController (Game|GetPlayerController 0)))
  (Utilities|IsValid (PlayerController|LocalPlayerSubsystems|GetEnhancedInputLocalPlayerSubsystem _asplayer_controller)
    (:Is%20Valid
      (Input|AddMappingContext (PlayerController|LocalPlayerSubsystems|GetEnhancedInputLocalPlayerSubsystem _asplayer_controller) "/Game/Input/PlayerControls.PlayerControls" 0 "(bIgnoreAllPressedKeysUntilRelease=True,bForceImmediately=False,bNotifyUserSettings=False)"))))

(fn SetupBaskets
  (Variables|Default|SetBaskets (Utilities|Array|MakeArray (Variables|Default|GetBasket%202) (Variables|Default|GetBasket%201) (Variables|Default|GetBasket%203))))