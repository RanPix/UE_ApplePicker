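; BP_Tree is an actor that slides back and forth along the X axis and drops BP_Apple actors.
; Tick advances two timers, moves the tree, then checks for turning and spawning.
; The tree reverses whenever outside its X bounds, or on a random per-frame roll once the direction-change cooldown has passed.
; An apple spawns at the tree's location each time the spawn timer exceeds its interval.
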(event EventBeginPlay)

(event Collision|EventActorBeginOverlap
  (params (OtherActor :type Actor%20Object%20Reference)))

(event EventTick
  (params (DeltaSeconds :type Float%20%28single-precision%29))
  (CallFunction|UpdateAppleSpawnTimer DeltaSeconds)
  (CallFunction|UpdateTreeDirectionChangeCDTimer DeltaSeconds)
  (CallFunction|Move DeltaSeconds)
  (CallFunction|TryChangeDirection)
  (CallFunction|TrySpawnApple))

(fn ConstructionScript)

(fn Move
  (params (Delta%20Seconds :type Float%20%28single-precision%29))
  (Transformation|SetActorLocation (+ (Math|Vector|MakeVector (* (* (Variables|Default|GetMoveDirection) (Variables|Default|GetSpeed)) Delta%20Seconds) 0.0 0.0) (Transformation|GetActorLocation)) false false))

(fn TryChangeDirection
  (bind _isoutofbounds (CallFunction|IsOutOfBounds))
  (if _isoutofbounds
    (CallFunction|ChangeDirection :!label _label)
    (elif (== 10 (Math|Random|RandomInteger 11))
      (bind _canchangedirection (CallFunction|CanChangeDirection))
      (if _canchangedirection
        (Variables|Default|SetTreeDirectionChangeCDTimer 0.0)
        (goto _label)))))

(fn UpdateAppleSpawnTimer
  (params (Delta%20Seconds :type Float%20%28double-precision%29))
  (Variables|Default|SetAppleSpawnTimer (+ Delta%20Seconds (Variables|Default|GetAppleSpawnTimer))))

(fn SpawnApple
  (Game|SpawnActorfromClass "/Game/Blueprints/BP_Apple.BP_Apple_C" (Math|Transform|MakeTransform (Transformation|GetActorLocation)) "Undefined" "MultiplyWithRoot" 0 0))

(fn TrySpawnApple
  (if (> (Variables|Default|GetAppleSpawnTimer) (Variables|Default|GetAppleSpawnTime))
    (CallFunction|SpawnApple)
    (Variables|Default|SetAppleSpawnTimer 0.0)))

(fn ChangeDirection
  (Variables|Default|SetMoveDirection (* -1.0 (Variables|Default|GetMoveDirection))))

(fn IsOutOfBounds
  (return (or (> (.x (Transformation|GetActorLocation)) (.y (Variables|Default|GetBounds))) (< (.x (Transformation|GetActorLocation)) (.x (Variables|Default|GetBounds))))))

(fn CanChangeDirection
  (return (> (Variables|Default|GetTreeDirectionChangeCDTimer) (Variables|Default|GetTreeDirectionChangeCDTime))))

(fn UpdateTreeDirectionChangeCDTimer
  (params (DeltaSeconds :type Float%20%28double-precision%29))
  (Variables|Default|SetTreeDirectionChangeCDTimer (+ DeltaSeconds (Variables|Default|GetTreeDirectionChangeCDTimer))))